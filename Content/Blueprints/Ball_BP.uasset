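; Ball actor for a brick-breaking game that destroys bricks it hits and counts points.
; The SM_Ball hit event plays a sound on every impact, then destroys any actor tagged Brick with a second sound.
; Each brick increments the ball's own Score and prints it; the AddPoints event it also calls is empty.
; Both sounds play at the world origin rather than the impact point.
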(event `self.SM_Ball.OnComponentHit`
  (params (HitComponent :type "PrimitiveComponent Object Reference") (OtherActor :type "Actor Object Reference") (OtherComp :type "PrimitiveComponent Object Reference") (NormalImpulse :type "Vector Structure") (Hit :type "HitResult Structure (by ref)"))
  (`GameplayStatics.PlaySoundAtLocation` "/Engine/VREditor/Sounds/UI/Laser_Pull.Laser_Pull" (0.0 0.0 0.0) (struct) 1.0 1.0 0.0 null null null)
  (if (`self.ActorHasTag` OtherActor "Brick")
    (`self.K2_DestroyActor` OtherActor)
    (`GameplayStatics.PlaySoundAtLocation` "/Engine/VREditor/Sounds/UI/Floating_UI_Open-002.Floating_UI_Open-002" (0.0 0.0 0.0) (struct) 1.0 1.0 0.0 null null null)
    (`self.AddPoints` 1)
    (bind _output_get (set `self.Score` (+ (`self.Score`) 1)))
    (`KismetSystemLibrary.PrintString` (`KismetStringLibrary.Conv_IntToString` _output_get))))

(event `AddPoints`
  (params (Score :type Integer :default 1)))

(fn `UserConstructionScript`)