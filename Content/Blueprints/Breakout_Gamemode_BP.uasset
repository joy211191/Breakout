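; Game mode for a Breakout game that keeps the current score and passes it to a UI widget.
; The UpdateScore event adds the incoming value to CurrentScore, clamps the total at zero and copies it to the Points variable of the Widget reference, which is not assigned in these graphs.
; BeginPlay only prints a level-start message, and Tick is unused.
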(event `self.ReceiveBeginPlay`
  (`KismetSystemLibrary.PrintString` "Level Started"))

(event `UpdateScore`
  (params (Score :type Integer))
  (bind _returnvalue (+ Score (`self.CurrentScore`)))
  (if (<= _returnvalue 0)
    (set `self.CurrentScore` 0)
    (else
      (set `self.CurrentScore` _returnvalue)))
  (set `/Game/Blueprints/Score.Points` (`self.CurrentScore`) (`self.Widget`)))

(fn `UserConstructionScript`)