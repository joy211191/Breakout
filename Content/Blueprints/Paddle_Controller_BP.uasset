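; Player controller for a brick-breaking paddle game that runs the score UI and the win condition.
; BeginPlay counts the Brick_BP actors and creates the HUD widget, and Tick pushes the ball count to it every frame.
; UpdateScore copies the score to the HUD and, when it equals the brick count, shows the win screen and cursor and tries to stop the ball, a step marked as not working.
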(event `self.ReceiveBeginPlay`
  (bind _outactors (`GameplayStatics.GetAllActorsOfClass` "/Game/Blueprints/Brick_BP.Brick_BP_C"))
  (set `self.NumberOfBricks` (`KismetArrayLibrary.Array_Length` _outactors))
  (bind _returnvalue (`|CreateWidget` "/Game/Blueprints/Score_UI.Score_UI_C"))
  (bind _output_get (set `self.UI` _returnvalue))
  (`UserWidget.AddToViewport` _output_get 0)
  (set `/Game/Blueprints/Score_UI.Balls` (`self.ballCount`) _output_get))

(event `self.ReceiveTick`
  (params (DeltaSeconds :type "Float (single-precision)"))
  ;[1 1 1] UI Update
  (set `/Game/Blueprints/Score_UI.Balls` (`self.ballCount`) (`self.UI`)))

(event `UpdateScore`
  ;[1 1 1] UI Update
  (bind _output_get (set `/Game/Blueprints/Score_UI.Score_UI` (`self.Score`) (`self.UI`)))
  ;[1 1 1] Game Win Screen
  (if (== _output_get (`self.NumberOfBricks`))
    (bind _returnvalue (`|CreateWidget` "/Game/Blueprints/GameWinScireen_BP.GameWinScireen_BP_C"))
    (`UserWidget.AddToViewport` _returnvalue 0)
    (set `self.bShowMouseCursor` true)
    ;[1 1 1] Freeze Ball (Not working)
    (bind _returnvalue_2 (`GameplayStatics.GetActorOfClass` "/Game/Blueprints/Ball_BP.Ball_BP_C"))
    (`ProjectileMovementComponent.SetVelocityInLocalSpace` (`Ball.ProjectileMovement` _returnvalue_2) (0.0 0.0 0.0))))

(fn `UserConstructionScript`)